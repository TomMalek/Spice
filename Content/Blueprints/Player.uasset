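; Player is a 2D side-view character Blueprint that moves along the X axis and displays flipbook animation.
; The MovePlayer axis adds movement input and sets controller yaw to face the direction of travel.
; Every tick, UpdateAnimation switches the sprite between walk and stand flipbooks based on whether velocity is non-zero.
; The JumpPlayer, LaunchCharacter and OnLanded events are empty, and a LaunchCharacter call sits unconnected, so jumping is not implemented here.
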(event `InputAxis|JumpPlayer`
  (params (AxisValue :type "Float (single-precision)")))

(event `Launch Character`)

(event `self.OnLanded`
  (params (Hit :type "HitResult Structure (by ref)")))

(event `InputAxis|MovePlayer`
  (params (AxisValue :type "Float (single-precision)"))
  (bind _returnvalue (`self.GetController`))
  ;[1 1 1] Movement
  (`self.AddMovementInput` (1.0 0.0 0.0) AxisValue)
  (`/Engine/EditorBlueprintResources/StandardMacros.CompareFloat` AxisValue
    (:`>`
      (`Controller.SetControlRotation` _returnvalue (`KismetMathLibrary.MakeRotator` 0.0)))
    (:`<`
      (`Controller.SetControlRotation` _returnvalue (`KismetMathLibrary.MakeRotator` 0.0 0.0 180.0)))))

(event `self.ReceiveTick`
  (params (DeltaSeconds :type "Float (single-precision)"))
  (`self.Update Animation`))

(event `Update Animation`
  ;[1 1 1] Animation
  (`PaperFlipbookComponent.SetFlipbook` (`self.Sprite`) (select `bool` (> (`KismetMathLibrary.VSize` (`self.GetVelocity`)) 0.0) :`false` "/Game/Flipbook/StandFlipbook/StandFlipbook.StandFlipbook" :`true` "/Game/Flipbook/WalkFlipbook/walkFlipbook.walkFlipbook" :!type "PaperFlipbook Object Reference")))

(fn `UserConstructionScript`)